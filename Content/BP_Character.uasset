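; BP_Character is a character Blueprint that lets the player grab objects and sprint through Enhanced Input actions.
; IA_Confirm calls Grab on a Grabber component when pressed and Release when let go.
; IA_Sprint calls StartSprint while triggered and StopSprint on completion, switching CharacterMovement MaxWalkSpeed between SprintSpeed and WalkSpeed.
; BeginPlay, overlap and Tick are unused stubs, and the construction script only calls its parent.
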(event Input|EnhancedActionEvents|EnhancedInputActionIA_Confirm
  (params (ActionValue :type Boolean) (ElapsedSeconds :type Float%20%28double-precision%29) (TriggeredSeconds :type Float%20%28double-precision%29) (InputAction :type Input%20Action%20Object%20Reference :default "/Game/Input/Actions/IA_Confirm.IA_Confirm"))
  (bind _grabber (Variables|Default|GetGrabber))
  (:Started
    (Class|Grabber|Grab _grabber))
  (:Completed
    (Class|Grabber|Release _grabber)))

(event Input|EnhancedActionEvents|EnhancedInputActionIA_Sprint
  (params (ActionValue :type Boolean) (ElapsedSeconds :type Float%20%28double-precision%29) (TriggeredSeconds :type Float%20%28double-precision%29) (InputAction :type Input%20Action%20Object%20Reference :default "/Game/Input/Actions/IA_Sprint.IA_Sprint"))
  (:Triggered
    (CallFunction|StartSprint))
  (:Completed
    (CallFunction|StopSprint)))

(event EventBeginPlay)

(event Collision|EventActorBeginOverlap
  (params (OtherActor :type Actor%20Object%20Reference)))

(event EventTick
  (params (DeltaSeconds :type Float%20%28single-precision%29)))

(fn ConstructionScript
  (|CallParentFunction))

(fn StartSprint
  (Variables|/Script/Engine.CharacterMovementComponent|SetMaxWalkSpeed (Variables|Character|GetCharacterMovement) (Variables|Default|GetSprintSpeed)))

(fn StopSprint
  (Variables|/Script/Engine.CharacterMovementComponent|SetMaxWalkSpeed (Variables|Character|GetCharacterMovement) (Variables|Default|GetWalkSpeed)))